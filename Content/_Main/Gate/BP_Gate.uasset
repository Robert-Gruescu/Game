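; BP_Gate is a gate actor that tilts as it is damaged and falls over once the damage passes a threshold.
; Each DestroyGate call increases GateAngle and adds it to the actor's roll until the limit is reached.
; Further calls play a timeline that rotates the gate toward 90 degrees roll, then disables mesh and box collision after a short delay.
; RepairGate lowers GateAngle and subtracts it from roll, without restoring collision.
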(event `/Game/_Main/Interfaces/DestroyGate.Destroy Gate`
  (bind (_returnvalue_roll _returnvalue_pitch _returnvalue_yaw) (`KismetMathLibrary.BreakRotator` (`self.K2_GetActorRotation`)))
  (bind (_returnvalue_roll_2 _returnvalue_pitch_2 _returnvalue_yaw_2) (`KismetMathLibrary.BreakRotator` (`self.K2_GetActorRotation`)))
  (if (< (`self.Gate Angle`) 2.0)
    (bind _output_get (set `self.Gate Angle` (+ (`self.Gate Angle`) 0.1)))
    (`self.K2_SetActorRotation` (`KismetMathLibrary.MakeRotator` (+ _output_get _returnvalue_roll_2) _returnvalue_pitch_2 _returnvalue_yaw_2))
    (else
      (`|ExecutionSequence`
        (:`then_0`
          (bind (_direction _newtrack_0) (`Timeline|Gate Falling TineLine`)
            (:`Update`
              (`self.K2_SetActorRotation` (`KismetMathLibrary.MakeRotator` (`KismetMathLibrary.MapRangeClamped` _newtrack_0 0.0 90.0 _returnvalue_roll 90.0) _returnvalue_pitch _returnvalue_yaw))
              (`KismetSystemLibrary.Delay` 0.5)
              (`PrimitiveComponent.SetCollisionEnabled` (`self.GateMesh`) "NoCollision")
              (`PrimitiveComponent.SetCollisionEnabled` (`self.Box`) "NoCollision")
              (`PrimitiveComponent.SetCollisionEnabled` (`self.GateMesh1`) "NoCollision"))))))))

(event `/Game/_Main/Interfaces/RepairGate.RepairGate`
  (bind (_returnvalue_roll _returnvalue_pitch _returnvalue_yaw) (`KismetMathLibrary.BreakRotator` (`self.K2_GetActorRotation`)))
  (bind _output_get (set `self.Gate Angle` (- (`self.Gate Angle`) 0.1)))
  (`self.K2_SetActorRotation` (`KismetMathLibrary.MakeRotator` (- _returnvalue_roll _output_get) _returnvalue_pitch _returnvalue_yaw)))

(fn `UserConstructionScript`)